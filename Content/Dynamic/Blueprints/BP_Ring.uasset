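; BP_Ring is a launch ring that flings the first-person character when it overlaps the ring's sphere.
; A dot product between the direction to the ring and the character mesh's forward vector tests whether the ring is ahead or behind.
; The character is launched at fixed speed along that forward vector, or its reverse, overriding current velocity on all axes.
; The ring's own orientation plays no part in the live logic.
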(event OnComponentBeginOverlap(Sphere)
  (params (OverlappedComponent :type Primitive%20Component%20Object%20Reference) (OtherActor :type Actor%20Object%20Reference) (OtherComp :type Primitive%20Component%20Object%20Reference) (OtherBodyIndex :type Integer) (bFromSweep :type Boolean) (SweepResult :type Hit%20Result%20Structure%20%28by%20ref%29))
  (bind _asbp_first_person_character (Utilities|Casting|CastToBP_FirstPersonCharacter OtherActor))
  (if (> (Math|Vector|DotProduct (Math|Vector|Normalize (- (Transformation|GetActorLocation (Components|GetOwner (Variables|Default|GetSphere))) (Transformation|GetActorLocation _asbp_first_person_character))) (Math|Vector|GetForwardVector (Variables|/Script/Engine.Character|GetMesh _asbp_first_person_character))) 0.0)
    (Character|LaunchCharacter _asbp_first_person_character (* (Math|Vector|GetForwardVector (Variables|/Script/Engine.Character|GetMesh _asbp_first_person_character)) 2e+03) true true)
    (else
      (Character|LaunchCharacter _asbp_first_person_character (* (Math|Vector|GetForwardVector (Variables|/Script/Engine.Character|GetMesh _asbp_first_person_character)) -2e+03) true true))))

(event EventBeginPlay)

(event Collision|EventActorBeginOverlap
  (params (OtherActor :type Actor%20Object%20Reference)))

(event EventTick
  (params (DeltaSeconds :type Float%20%28single-precision%29)))

(fn ConstructionScript)