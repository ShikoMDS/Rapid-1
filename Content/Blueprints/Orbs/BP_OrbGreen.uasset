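; BP_OrbGreen is a collectible green orb that boosts the first-person player and awards two points when touched.
; An overlap on its mesh with BP_FirstPersonCharacter launches the character along the camera's forward vector, adding to its current velocity.
; It then adds to the Score in BP_FirstPersonGameMode, destroys itself and prints the new score.
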(event OnComponentBeginOverlap(OrbMesh)
  (params (OverlappedComponent :type Primitive%20Component%20Object%20Reference) (OtherActor :type Actor%20Object%20Reference) (OtherComp :type Primitive%20Component%20Object%20Reference) (OtherBodyIndex :type Integer) (bFromSweep :type Boolean) (SweepResult :type Hit%20Result%20Structure%20%28by%20ref%29))
  (bind _asbp_first_person_character (Utilities|Casting|CastToBP_FirstPersonCharacter OtherActor))
  (Character|LaunchCharacter _asbp_first_person_character (* (Math|Vector|GetForwardVector (Variables|/Game/Dynamic/FirstPerson/Blueprints/BP_FirstPersonCharacter.BP_FirstPersonCharacter_C|GetFirstPersonCamera _asbp_first_person_character)) 1e+03) false false)
  (CallFunction|CollectOrb))

(event Custom|CollectOrb
  (bind _asbp_first_person_game_mode (Utilities|Casting|CastToBP_FirstPersonGameMode (Game|GetGameMode)))
  (bind _output_get (Variables|/Game/Dynamic/FirstPerson/Blueprints/BP_FirstPersonGameMode.BP_FirstPersonGameMode_C|SetScore _asbp_first_person_game_mode (+ (Variables|/Game/Dynamic/FirstPerson/Blueprints/BP_FirstPersonGameMode.BP_FirstPersonGameMode_C|GetScore _asbp_first_person_game_mode) 2)))
  (Actor|DestroyActor)
  (Development|PrintString (Utilities|String|ToString(Integer) _output_get)))

(event EventBeginPlay)

(event Collision|EventActorBeginOverlap
  (params (OtherActor :type Actor%20Object%20Reference)))

(fn ConstructionScript)